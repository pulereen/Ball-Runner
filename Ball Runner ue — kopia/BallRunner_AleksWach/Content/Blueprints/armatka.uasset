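; Cannon actor that automatically and repeatedly fires Pocisk projectiles from the moment play begins.
; After a short delay it spawns a projectile at the Arrow component's world transform, then plays the CannonLocation timeline to move the Cannon component along its relative Y axis.
; The timeline's Finished output loops back to the delay, so firing continues indefinitely.
; A CannonAnimation function holds the same relative-location update but is not called in this graph.
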(event EventBeginPlay
  (bind _arrow (Variables|Default|GetArrow))
  (Utilities|FlowControl|Delay 0.2 :!label _label)
  (Game|SpawnActorfromClass "/Game/Projectiles/Pocisk.Pocisk_C" (Math|Transform|MakeTransform (Transformation|GetWorldLocation _arrow) (Transformation|GetWorldRotation _arrow) "1,1,1") "Undefined" 0 0)
  (bind _newtrack_0 (Timeline|CannonLocation PlayFromStart)
    (:Update
      (Transformation|SetRelativeLocation (Variables|Default|GetCannon) (Math|Vector|MakeVector 0.0 _newtrack_0 0.0) false false))
    (:Finished
      (goto _label))))

(fn ConstructionScript)

(fn CannonAnimation
  (params (NewLocation%20Y :type Float%20%28single-precision%29))
  (Transformation|SetRelativeLocation (Variables|Default|GetCannon) (Math|Vector|MakeVector 0.0 NewLocation%20Y 0.0) false false))
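; Player-controlled ball that moves by applying torque to its static mesh.
; Forward/backward and left/right input axes drive torque around X and Y as an acceleration change, so the spin is independent of mass.
; Each axis event first calls CheckInput, which re-applies game-only input mode and enables input for the first player controller.
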(event Input|AxisEvents|InputAxisMoveForward/Backwards
  (params (AxisValue :type Float%20%28single-precision%29))
  (CallFunction|CheckInput)
  (Class|PrimitiveComponent|AddTorqueinRadians (Variables|Default|GetStaticMesh) (Math|Vector|MakeVector (* AxisValue 3e+01) 0.0 0.0) "None" true))

(event Input|AxisEvents|InputAxisMoveLeft/Right
  (params (AxisValue :type Float%20%28single-precision%29))
  (CallFunction|CheckInput)
  (Class|PrimitiveComponent|AddTorqueinRadians (Variables|Default|GetStaticMesh) (Math|Vector|MakeVector 0.0 (* AxisValue 3e+01) 0.0) "None" true))

(fn ConstructionScript)

(fn CheckInput
  (bind _returnvalue (Game|GetPlayerController 0))
  (Input|SetInputModeGameOnly _returnvalue)
  (Input|EnableInput _returnvalue))